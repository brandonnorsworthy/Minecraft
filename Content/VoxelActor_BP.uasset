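; VoxelActor_BP is a voxel chunk actor that supplies an integer noise map, apparently terrain heights, for its grid cell.
; CalculateNoise walks the chunk's columns row by row, offsetting by chunk index so sampling uses continuous world grid coordinates.
; It sums four weighted simplex noise octaves, clamping the finest to non-negative values, then truncates into the Noise array.
; Event and construction graphs are empty, and a frequency test branch is disconnected.
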(event EventBeginPlay)

(event Collision|EventActorBeginOverlap
  (params (OtherActor :type Actor%20Object%20Reference)))

(event EventTick
  (params (DeltaSeconds :type Float%20%28single-precision%29)))

(fn ConstructionScript)

(fn CalculateNoise
  (bind _chunklineelements (Variables|Default|GetchunkLineElements))
  (bind _returnvalue (- _chunklineelements 1))
  (for _index (range 0 _returnvalue)
    (LocalVariables|SetyLoc _index)
    (for _index_2 (range 0 _returnvalue)
      (LocalVariables|SetxLoc _index_2)
      (bind _returnvalue_2 (Class|SimplexNoiseBPLibrary|SimplexNoise2D (* (+ (LocalVariables|GetxLoc) (* (Variables|Default|GetchunkXindex) (Variables|Default|GetchunkLineElements))) 1.0) (* (+ (LocalVariables|GetyLoc) (* (Variables|Default|GetchunkYIndex) (Variables|Default|GetchunkLineElements))) 1.0) 0.01))
      (bind _returnvalue_3 (Class|SimplexNoiseBPLibrary|SimplexNoise2D (* (+ (LocalVariables|GetxLoc) (* (Variables|Default|GetchunkXindex) (Variables|Default|GetchunkLineElements))) 1.0) (* (+ (LocalVariables|GetyLoc) (* (Variables|Default|GetchunkYIndex) (Variables|Default|GetchunkLineElements))) 1.0) 0.005))
      (bind _returnvalue_4 (Class|SimplexNoiseBPLibrary|SimplexNoise2D (* (+ (LocalVariables|GetxLoc) (* (Variables|Default|GetchunkXindex) (Variables|Default|GetchunkLineElements))) 2.0) (* (+ (LocalVariables|GetyLoc) (* (Variables|Default|GetchunkYIndex) (Variables|Default|GetchunkLineElements))) 2.0) 0.001))
      (bind _returnvalue_5 (Class|SimplexNoiseBPLibrary|SimplexNoise2D (* (+ (LocalVariables|GetxLoc) (* (Variables|Default|GetchunkXindex) (Variables|Default|GetchunkLineElements))) 1.0) (* (+ (LocalVariables|GetyLoc) (* (Variables|Default|GetchunkYIndex) (Variables|Default|GetchunkLineElements))) 1.0) 0.05))
      (Utilities|Array|Add (LocalVariables|GetNoise) (Math|Float|Truncate (+ (* _returnvalue_2 4.0) (* _returnvalue_3 1e+01) (* _returnvalue_4 16.0) (Math|Float|Clamp(Float) (* _returnvalue_5 4.0) 0.0 4.0))))))
  (return (LocalVariables|GetNoise)))