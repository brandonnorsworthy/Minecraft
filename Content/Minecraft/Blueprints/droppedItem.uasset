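; Dropped Minecraft-style block item that bobs and spins via a timeline, with its material chosen by ItemID in the construction script.
; Tick finds nearby matching items, recalculates only its own BlockQuantity against a 64 limit, then calls UpdateMesh on both.
; UpdateMesh holds tiered visibility for stacked block meshes, but its first check destroys any item with quantity one or more, leaving those tiers unreachable.
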(event Custom|Update%20Mesh
  (bind _block3 (Variables|Default|Getblock3))
  (bind _block4 (Variables|Default|Getblock4))
  (bind _block5 (Variables|Default|Getblock5))
  (bind _block2 (Variables|Default|Getblock2))
  (if (< (Variables|Default|GetblockQuantity) 1)
    (if (< 1 (Variables|Default|GetblockQuantity))
      (Rendering|SetVisibility _block2 true false)
      (if (< 16 (Variables|Default|GetblockQuantity))
        (Rendering|SetVisibility _block3 true false)
        (if (< 32 (Variables|Default|GetblockQuantity))
          (Rendering|SetVisibility _block4 true false)
          (if (< 48 (Variables|Default|GetblockQuantity))
            (Rendering|SetVisibility _block5 true false)
            (else
              (Rendering|SetVisibility _block5 false false :!label _label)))
          (else
            (Rendering|SetVisibility _block4 false false :!label _label_2)
            (goto _label)))
        (else
          (Rendering|SetVisibility _block3 false false :!label _label_3)
          (goto _label_2)))
      (else
        (Rendering|SetVisibility _block2 false false)
        (goto _label_3)))
    (else
      (Actor|DestroyActor))))

(event Custom|Play%20Animation
  (bind _block1 (Variables|Components|Getblock1))
  (bind _returnvalue (Transformation|GetWorldLocation _block1))
  (bind (_direction _z _rotation) (Timeline|RotateAnimation Play)
    (:Update
      (Transformation|SetWorldLocation _block1 (Math|Vector|MakeVector (.x _returnvalue) (.y _returnvalue) (+ (.z _returnvalue) (* _z 0.1))) false false)
      (Transformation|SetWorldRotation _block1 (Math|Rotator|MakeRotator 0.0 0.0 _rotation) false false))))

(event EventTick
  (params (DeltaSeconds :type Float%20%28single-precision%29))
  (bind (_outactors _returnvalue) (Collision|SphereOverlapActors (Transformation|GetActorLocation) 1.5e+02 (Utilities|Array|MakeArray "ObjectTypeQuery2") "droppedItem_C" (Utilities|Array|MakeArray self)))
  (if _returnvalue
    (for _array_element _outactors
      (bind _asdropped_item (Utilities|Casting|CastTodroppedItem _array_element))
      (if (== (Variables|Default|GetitemID) (Variables|droppedItem_C|GetitemID _asdropped_item))
        (if (>= (Variables|Default|GetblockQuantity) (Variables|droppedItem_C|GetblockQuantity _asdropped_item))
          (Variables|Default|SetblockQuantity (- (- 64 (Variables|Default|GetblockQuantity)) (Variables|droppedItem_C|GetblockQuantity _asdropped_item)))
          (CallFunction|UpdateMesh _asdropped_item)
          (CallFunction|UpdateMesh))))))

(fn ConstructionScript
  (CallFunction|ApplyMaterialtoAll (Utilities|Select :Index (Variables|Default|GetitemID) :Option%200 "/Game/Minecraft/Blocks/Materials/devmaterial.devmaterial" :Option%201 "/Game/Minecraft/Blocks/Materials/grass_block_Mat.grass_block_Mat" :Option%202 "/Game/Minecraft/Blocks/Materials/dirt_Mat.dirt_Mat" :Option%203 "/Game/Minecraft/Blocks/Materials/stone_Mat.stone_Mat" :Option%204 "/Game/Minecraft/Blocks/Materials/devmaterial.devmaterial" :Option%205 "/Game/Minecraft/Blocks/Materials/devmaterial.devmaterial" :Option%206 "/Game/Minecraft/Blocks/Materials/devmaterial.devmaterial" :Option%207 "/Game/Minecraft/Blocks/Materials/devmaterial.devmaterial" :Option%208 "/Game/Minecraft/Blocks/Materials/devmaterial.devmaterial" :Option%209 "/Game/Minecraft/Blocks/Materials/devmaterial.devmaterial" :Option%2010 "/Game/Minecraft/Blocks/Materials/devmaterial.devmaterial" :Option%2011 "/Game/Minecraft/Blocks/Materials/devmaterial.devmaterial" :Option%2012 "/Game/Minecraft/Blocks/Materials/devmaterial.devmaterial" :Option%2013 "/Game/Minecraft/Blocks/Materials/devmaterial.devmaterial" :Option%2014 "/Game/Minecraft/Blocks/Materials/devmaterial.devmaterial" :Option%2015 "/Game/Minecraft/Blocks/Materials/devmaterial.devmaterial" :Option%2016 "/Game/Minecraft/Blocks/Materials/devmaterial.devmaterial" :Option%2017 "/Game/Minecraft/Blocks/Materials/devmaterial.devmaterial" :Option%2018 "/Game/Minecraft/Blocks/Materials/devmaterial.devmaterial" :Option%2019 "/Game/Minecraft/Blocks/Materials/devmaterial.devmaterial" :Option%2020 "/Game/Minecraft/Blocks/Materials/testleaves_Mat.testleaves_Mat" :Option%2021 "/Game/Minecraft/Blocks/Materials/oak_log_Mat.oak_log_Mat"))
  (CallFunction|PlayAnimation))

(fn ApplyMaterialtoAll
  (params (Material :type Material%20Object%20Reference))
  (Rendering|Material|SetMaterial (Variables|Components|Getblock1) 0 Material)
  (Rendering|Material|SetMaterial (Variables|Default|Getblock2) 0 Material)
  (Rendering|Material|SetMaterial (Variables|Default|Getblock3) 0 Material)
  (Rendering|Material|SetMaterial (Variables|Default|Getblock4) 0 Material)
  (Rendering|Material|SetMaterial (Variables|Default|Getblock5) 0 Material))